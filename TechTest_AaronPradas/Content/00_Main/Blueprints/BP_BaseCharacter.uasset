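; BP_BaseCharacter is a base character Blueprint that manages a single Stamina resource.
; Stamina starts at MaxStamina on BeginPlay, and the ApplyDamage and ApplyHealing events lower or raise it through SetStamina.
; SetStamina clamps the value between zero and MaxStamina, then fires OnStaminaChanged, while GetStaminaPercent returns the current ratio.
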(event `self.ReceiveBeginPlay`
  ;[1 0.7798 0.276 0.5] BEGIN PLAY
  (set `self.Stamina` (`self.MaxStamina`)))

(event `/Game/00_Main/Blueprints/BPI_Damage.ApplyDamage`
  (params (Amount :type "Float (double-precision)"))
  (`self.SetStamina` (- (`self.Stamina`) Amount)))

(event `/Game/00_Main/Blueprints/BPI_Damage.ApplyHealing`
  (params (Amount :type "Float (double-precision)"))
  (`self.SetStamina` (+ (`self.Stamina`) Amount)))

(fn `GetStaminaPercent`
  (returns (StaminaPercent :type "Float (double-precision)"))
  (return (/ (`self.Stamina`) (`self.MaxStamina`))))

(fn `SetStamina`
  (params (NewStamina :type "Float (double-precision)"))
  (set `self.Stamina` (`KismetMathLibrary.FClamp` NewStamina 0.0 (`self.MaxStamina`)))
  (`self.OnStaminaChanged`))

(fn `UserConstructionScript`)