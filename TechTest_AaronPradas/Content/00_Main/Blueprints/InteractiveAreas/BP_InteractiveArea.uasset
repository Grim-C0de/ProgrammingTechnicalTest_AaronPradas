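; Base interactive area that periodically applies an effect to overlapping actors implementing BPI_Damage.
; Collision overlaps maintain the affected-actor list, starting a looping timer at EffectRate on entry and clearing it once the list empties.
; AffectOverlappedActors passes each listed actor to ApplyEffect, which is empty here.
; The construction script tints the cube with the configurable Color.
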(event `StartEffects`
  (if (not (`KismetSystemLibrary.K2_IsTimerActiveHandle` (`self.TH_ApplyEffects`)))
    (bind _returnvalue (`KismetSystemLibrary.K2_SetTimerDelegate` (`|CreateDelegate` :!event `AffectOverlappedActors`) (`self.EffectRate`) true))
    (set `self.TH_ApplyEffects` _returnvalue)))

(event `self.Collision.OnComponentBeginOverlap`
  (params (OverlappedComponent :type "PrimitiveComponent Object Reference") (OtherActor :type "Actor Object Reference") (OtherComp :type "PrimitiveComponent Object Reference") (OtherBodyIndex :type Integer) (bFromSweep :type Boolean) (SweepResult :type "HitResult Structure (by ref)"))
  (bind _asbpi_damage (cast `/Game/00_Main/Blueprints/BPI_Damage` OtherActor))
  (`KismetArrayLibrary.Array_AddUnique` (`self.AffectedActors`) _asbpi_damage)
  (`self.StartEffects`))

(event `self.Collision.OnComponentEndOverlap`
  (params (OverlappedComponent :type "PrimitiveComponent Object Reference") (OtherActor :type "Actor Object Reference") (OtherComp :type "PrimitiveComponent Object Reference") (OtherBodyIndex :type Integer))
  (bind _affectedactors (`self.AffectedActors`))
  (bind _asbpi_damage (cast `/Game/00_Main/Blueprints/BPI_Damage` OtherActor))
  (`KismetArrayLibrary.Array_RemoveItem` _affectedactors _asbpi_damage)
  (if (`KismetArrayLibrary.Array_IsEmpty` _affectedactors)
    (`KismetSystemLibrary.K2_ClearAndInvalidateTimerHandle` (`self.TH_ApplyEffects`))))

(fn `AffectOverlappedActors`
  (for _array_element (`self.AffectedActors`)
    (`self.ApplyEffect` _array_element)))

(fn `ApplyEffect`
  (params (Damage :type "/Game/00_Main/Blueprints/BPI_Damage Interface")))

(fn `UserConstructionScript`
  (`MeshComponent.SetColorParameterValueOnMaterials` (`self.Cube`) "Color" (`self.Color`)))