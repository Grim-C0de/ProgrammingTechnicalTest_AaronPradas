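; BP_EnemyDummy is a dummy enemy that shows its stamina on a widget-based bar.
; On BeginPlay it runs the parent logic, caches its WBP_EnemyHP widget, binds to the stamina-changed dispatcher and triggers an initial update.
; The handler sets the widget's HealthBar to the stamina percent, so the bar named for health tracks stamina.
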(event `self.ReceiveBeginPlay`
  ;[1 0.7798 0.276 0.5] BEGIN PLAY
  (`parent.ReceiveBeginPlay`)
  (bind _aswbp_enemy_hp (cast `/Game/00_Main/Blueprints/Enemies/WBP_EnemyHP` (`WidgetComponent.GetWidget` (`self.Widget`))))
  (set `self.W_EnemyHP` _aswbp_enemy_hp)
  (add `self.OnStaminaChanged` (`|CreateDelegate` :!event `OnStaminaChanged_Event`))
  (`self.OnStaminaChanged_Event`))

(event `OnStaminaChanged_Event`
  (bind _w_enemyhp (`self.W_EnemyHP`)
    (:`then`
      (`ProgressBar.SetPercent` (`/Game/00_Main/Blueprints/Enemies/WBP_EnemyHP.HealthBar` _w_enemyhp) (`self.GetStaminaPercent`)))
    (:`else`)))

(fn `UserConstructionScript`)